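; Character Blueprint with life-sim style needs (hunger, thirst, health, hygiene, sleep) and click-to-move navigation.
; BeginPlay starts a looping one-second timer, presumably driving Statupdate, though the bound event is not shown.
; Statupdate decrements all five current need values together, with no clamping or reaction to depletion.
; Gototheclick sends the controller to a supplied destination through SimpleMoveToLocation.
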(event Custom|Go%20to%20the%20click
  (params (Destination :type Vector))
  ;[1 1 1] Go to click
  (AI|Navigation|SimpleMovetoLocation (Pawn|GetController) Destination))

(event Custom|Stat%20update
  ;[1 1 1] Stat update
  (Math|Integer|DecrementInt (Variables|Statistique|GetFaim%20actuel)
    (:%20%20
      (Math|Integer|DecrementInt (Variables|Statistique|Getsoif%20actuel)
        (:%20%20
          (Math|Integer|DecrementInt (Variables|Statistique|GetSante%20actuel)
            (:%20%20
              (Math|Integer|DecrementInt (Variables|Statistique|Gethygiene%20actuel)
                (:%20%20
                  (Math|Integer|DecrementInt (Variables|Statistique|Getsommeil%20actuel)))))))))))

(event EventBeginPlay
  ;[1 1 1] Event begin play
  (Utilities|Time|SetTimerbyEvent (EventDispatchers|CreateEvent :!event Custom|Stat%20update) 1.0 true))

(fn ConstructionScript)